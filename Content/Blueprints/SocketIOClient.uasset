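; Actor that hosts a multiplayer submarine game session over Socket.IO, letting remote clients control submarines through a Heroku relay server.
; On BeginPlay it creates a session; join and left events spawn submarines at random points or destroy them, using a map keyed by sender ID.
; Input events set the sender's rotation and velocity and trigger submerge, mine, torpedo or missile actions.
; Each handled input also emits players' lives back as JSON via SendHearts.
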(event `ReceiveCreated`
  (params (Message :type String))
  (`KismetSystemLibrary.PrintString` Message))

(event `self.ReceiveBeginPlay`
  (bind _socketioclient (`self.SocketIOClient`))
  (set `self.players` (`|MakeMap`))
  (`SocketIOClientComponent.Connect` _socketioclient "ws://seawolf-server.herokuapp.com/" null null)
  (`SocketIOClientComponent.BindEventToFunction` _socketioclient "created" "ReceiveCreated" null "/" "USE_DEFAULT")
  (`SocketIOClientComponent.Emit` _socketioclient "create" null "/")
  (`SocketIOClientComponent.BindEventToFunction` _socketioclient "join" "PlayerJoined" null "/" "USE_DEFAULT")
  (`SocketIOClientComponent.BindEventToFunction` _socketioclient "left" "PlayerLeft" null "/" "USE_DEFAULT")
  (`SocketIOClientComponent.BindEventToFunction` _socketioclient "input" "ReceivedInput" null "/" "USE_DEFAULT"))

(event `ReceivedInput`
  (params (NewParam :type "SIOJsonObject Object Reference"))
  (bind _returnvalue (`SIOJLibrary.Conv_JsonValueToJsonObject` (`SIOJsonObject.GetField` NewParam "data")))
  (bind (_value _returnvalue_2) (`BlueprintMapLibrary.Map_Find` (`self.players`) (`SIOJsonValue.AsString` (`SIOJsonObject.GetField` NewParam "from"))))
  (bind _returnvalue_3 (`KismetMathLibrary.RadiansToDegrees` (`SIOJsonValue.AsNumber` (`SIOJsonObject.GetField` _returnvalue "direction"))))
  (if _returnvalue_2
    (`self.SendHearts`)
    (if (`SIOJsonValue.AsBool` (`SIOJsonObject.GetField` _returnvalue "submergeSwitch"))
      (`/Game/Blueprints/Submarine.Submerge` _value))
    (if (`SIOJsonValue.AsBool` (`SIOJsonObject.GetField` _returnvalue "sendBomb"))
      (`/Game/Blueprints/Submarine.Eject Mine` _value))
    (if (`SIOJsonValue.AsBool` (`SIOJsonObject.GetField` _returnvalue "sendTorpedo"))
      (`/Game/Blueprints/Submarine.Fire Torpedo` _value))
    (if (`SIOJsonValue.AsBool` (`SIOJsonObject.GetField` _returnvalue "sendMissile"))
      (`/Game/Blueprints/Submarine.Fire Missile` _value))
    (`self.K2_SetActorRotation` _value (`KismetMathLibrary.RotatorFromAxisAndAngle` (0.0 0.0 1.0) _returnvalue_3) false)
    (set `/Game/Blueprints/Submarine.Velocity` (* (* (`KismetMathLibrary.RotateAngleAxis` (1.0 0.0 0.0) _returnvalue_3 (0.0 0.0 1.0)) (`SIOJsonValue.AsNumber` (`SIOJsonObject.GetField` _returnvalue "magnitude"))) -100.0) _value)))

(event `PlayerJoined`
  (params (NewParam :type "SIOJsonObject Object Reference"))
  (bind _returnvalue (`SIOJsonValue.AsString` (`SIOJsonObject.GetField` NewParam "from")))
  (`KismetSystemLibrary.PrintString` (`KismetStringLibrary.Concat_StrStr` _returnvalue " has joined the game"))
  (bind _returnvalue_2 (`|SpawnActorFromClass` "/Game/Blueprints/Submarine.Submarine_C" (`self.generateSpawnPoint`) "Undefined" "OverrideRootScale" null null))
  (`BlueprintMapLibrary.Map_Add` (`self.players`) _returnvalue _returnvalue_2))

(event `PlayerLeft`
  (params (NewParam :type "SIOJsonObject Object Reference"))
  (bind _returnvalue (`SIOJsonValue.AsString` (`SIOJsonObject.GetField` NewParam "from")))
  (bind (_value _returnvalue_2) (`BlueprintMapLibrary.Map_Find` (`self.players`) _returnvalue))
  (`KismetSystemLibrary.PrintString` (`KismetStringLibrary.Concat_StrStr` _returnvalue " has left the game"))
  (if _returnvalue_2
    (`self.K2_DestroyActor` _value)))

(event `self.SocketIOClient.OnConnected`
  (params (SessionId :type String) (bIsReconnection :type Boolean))
  (`KismetSystemLibrary.PrintString` SessionId))

(fn `created`
  (params (NewParam :type Boolean)))

(fn `generateSpawnPoint`
  (returns (`Spawn Point` :type "Transform Structure"))
  (bind _output_get (set `self.Spawn Point` (`KismetMathLibrary.MakeVector` (`KismetMathLibrary.RandomFloatInRange` -250.0 250.0) (`KismetMathLibrary.RandomFloatInRange` -250.0 250.0))))
  (return (`KismetMathLibrary.MakeTransform` _output_get)))

(fn `SendHearts`
  (bind _players (`self.players`))
  (bind _keys (`BlueprintMapLibrary.Map_Keys` _players))
  (bind _returnvalue (`SIOJsonObject.ConstructJsonObject`))
  (for _array_element _keys
    (bind _returnvalue_2 (`SIOJsonObject.ConstructJsonObject`))
    (bind (_value _returnvalue_3) (`BlueprintMapLibrary.Map_Find` _players _array_element))
    (`SIOJsonObject.SetField` _returnvalue_2 "lives" (`SIOJLibrary.Conv_IntToJsonValue` (`/Game/Blueprints/Submarine.Current Lives` _value)))
    (`SIOJsonObject.SetObjectField` _returnvalue (`KismetStringLibrary.Conv_IntToString` (`KismetStringLibrary.Conv_StringToInt` _array_element)) _returnvalue_2)
    (if _returnvalue_3
      (`SocketIOClientComponent.Emit` (`self.SocketIOClient`) "data" (`SIOJLibrary.Conv_JsonObjectToJsonValue` _returnvalue) "/"))))

(fn `UserConstructionScript`)